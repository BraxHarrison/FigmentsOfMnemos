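; Game mode for the garden system, holding owned gardens and inventory and switching between overworld and Figment focus.
; BeginPlay seeds placeholder data through DEV functions: a garden containing one hard-coded Harshmallow Figment and a stock of fruit items.
; Figment focus spawns a Garden_BP from the garden and Figment structs and makes it the player's view target.
; Overworld focus only destroys that actor, without explicitly resetting the view target.
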(event `self.ReceiveBeginPlay`
  (`self.[DEV]InitBasicGarden`)
  (`self.[DEV]InitInventory`))

(fn `[DEV]InitBasicGarden`
  (`KismetSystemLibrary.PrintString` "YOB")
  (bind _figment (`self.createFigment`))
  (bind _output_get (set `self.gardenInfo` (make `/Game/System/Types/Garden_STRUCT` "Yob" "/Game/Maps/GrassyField/GrassyField_OVER.GrassyField_OVER" null (`|MakeArray` _figment))))
  (`KismetArrayLibrary.Array_Add` (`self.GardensOwned`) _output_get))

(fn `[DEV]InitInventory`
  (for _ (range 11)
    (`KismetArrayLibrary.Array_Add` (`self.inventory`) (make `/Game/System/Types/Item_STRUCT` "Some Fruit" "NewEnumerator0" "NewEnumerator0" "NewEnumerator0" 1.0 "/Game/Actors/Items/001_SomeFruit/SomeFruit.SomeFruit" "/Game/Actors/Items/001_SomeFruit/SomeFruit_SPRITE.SomeFruit_SPRITE"))))

(fn `createFigment`
  (returns (figment :type "/Game/System/Types/Figment_STRUCT Structure"))
  (locals (figmentName :type String))
  (bind _output_get (set `local.figmentName` "Harshmallow"))
  (return (make `/Game/System/Types/Figment_STRUCT` _output_get (`|MakeMap` "Stamina" 10) (`|MakeMap` "Stamina" "A") "/Game/Actors/Figments/001_Harshmallow/Harshmallow.Harshmallow" "/Game/Actors/Figments/001_Harshmallow/Anims/Harshmallow_AB.Harshmallow_AB_C" "/Game/Actors/Figments/001_Harshmallow/Harshmallow_SPRITE.Harshmallow_SPRITE" "/Game/Actors/GenericMaterial_MAT.GenericMaterial_MAT" "/Game/Actors/Figments/001_Harshmallow/Harshmallow_TEX.Harshmallow_TEX")))

(fn `swapToFigmentFocus`
  (params (playerController :type "/Game/System/Control/PC_Garden Object Reference") (figment :type "/Game/System/Types/Figment_STRUCT Structure (by ref)"))
  (bind _returnvalue (`|SpawnActorFromClass` "/Game/Maps/Garden_BP.Garden_BP_C" (`KismetMathLibrary.MakeTransform` (0.0 0.0 0.0)) "Undefined" "OverrideRootScale" null (`self.gardenInfo`) figment null))
  (`PlayerController.SetViewTargetWithBlend` playerController _returnvalue 0.0 "VTBlend_Linear" 0.0 false)
  (set `self.instantiatedGarden` _returnvalue))

(fn `swapToOverworldFocus`
  (`self.K2_DestroyActor` (`self.instantiatedGarden`)))

(fn `UserConstructionScript`)