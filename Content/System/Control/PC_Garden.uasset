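; Player controller for the garden scene that manages its touch UI and switches between overworld and Figment focus views.
; On BeginPlay it caches the GM_Garden game mode and creates both focus widgets, showing the overworld one.
; Tick turns touch movement past a threshold into screen drags on the overworld widget while no Figment is focused.
; Focusing a Figment notifies the game mode and swaps widgets; returning rebuilds the overworld widget.
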(event `self.ReceiveBeginPlay`
  ;[1 1 1] Set up UI on Playercontroller startup
  (`self.setGM`)
  (`self.initUI`))

(event `self.ReceiveTick`
  (params (DeltaSeconds :type "Float (single-precision)"))
  (bind (_locationx _locationy _biscurrentlypressed) (`self.GetInputTouchState` "Touch1"))
  (bind _returnvalue (`KismetMathLibrary.MakeVector2D` _locationx _locationy))
  ;[1 1 1] Handle Screen drag input
  (if (and (not (`self.figmentFocused?`)) _biscurrentlypressed)
    (if (>= (`KismetMathLibrary.VSize2D` (- _returnvalue (`self.startTouchLoc`))) (`self.dragThreshold`))
      (`|ExecutionSequence`
        (:`then_0`
          (`/Engine/EditorBlueprintResources/StandardMacros.DoOnce` true :!label _label
            (:`Completed`
              (set `self.startTouchLoc` _returnvalue))))
        (:`then_1`
          (`/Game/Maps/UI/OverworldFocus_UI.dragScreen` (`self.OverworldGUI`) (* (- _returnvalue (`self.startTouchLoc`)) (`self.dragSpeed`))))))
    (else
      (`/Game/Maps/UI/OverworldFocus_UI.finishDrag` (`self.OverworldGUI`))
      (goto _label :!via `Reset`))))

(fn `initUI`
  (bind _returnvalue (`|CreateWidget` "/Game/Maps/UI/OverworldFocus_UI.OverworldFocus_UI_C" self self (`/Game/Maps/Garden_BP.gardenInfo` (`/Game/System/Flow/GM_Garden.currentGarden` (`self.GameMode`)))))
  (bind _output_get (set `self.OverworldGUI` _returnvalue))
  (`UserWidget.AddToPlayerScreen` _output_get 0)
  (bind _returnvalue_2 (`|CreateWidget` "/Game/Maps/UI/FigmentFocus_UI.FigmentFocus_UI_C" null self))
  (set `self.FigmentFocusGUI` _returnvalue_2))

(fn `setGM`
  (bind _asgm_garden (cast `/Game/System/Flow/GM_Garden` (`GameplayStatics.GetGameMode`)))
  (set `self.GameMode` _asgm_garden))

(fn `triggerFigmentFocus`
  (params (figment :type "/Game/System/Flow/Figment_STRUCT Structure (by ref)"))
  (`/Game/System/Flow/GM_Garden.swapToFigmentFocus` (`self.GameMode`) self)
  (`Widget.RemoveFromParent` (`self.OverworldGUI`))
  (`UserWidget.AddToViewport` (`self.FigmentFocusGUI`) 0)
  (set `self.figmentFocused?` true))

(fn `triggerOverworldFocus`
  (`Widget.RemoveFromParent` (`self.FigmentFocusGUI`))
  (bind _returnvalue (`|CreateWidget` "/Game/Maps/UI/OverworldFocus_UI.OverworldFocus_UI_C" self self (`/Game/Maps/Garden_BP.gardenInfo` (`/Game/System/Flow/GM_Garden.currentGarden` (`self.GameMode`)))))
  (set `self.figmentFocused?` false)
  (`UserWidget.AddToPlayerScreen` _returnvalue 0)
  (set `self.OverworldGUI` _returnvalue))

(fn `UserConstructionScript`)