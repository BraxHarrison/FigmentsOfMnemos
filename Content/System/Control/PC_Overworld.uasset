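; Player controller for the overworld that creates the Overworld UI widget and turns touch input into screen dragging.
; Tick polls the first touch, latches its start location through a DoOnce, passes the offset to the widget's DragScreen, and calls FinishDrag whenever untouched.
; MoveCamera maps a drag vector to the sprite viewer's X/Z location, but the nodes that spawn and view that actor are disconnected.
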(event `self.ReceiveBeginPlay`
  (`self.initUI`))

(event `self.ReceiveTick`
  (params (DeltaSeconds :type "Float (single-precision)"))
  (bind (_locationx _locationy _biscurrentlypressed) (`self.GetInputTouchState` "Touch1"))
  (bind _returnvalue (`KismetMathLibrary.MakeVector2D` _locationx _locationy))
  (if _biscurrentlypressed
    (`|ExecutionSequence`
      (:`then_0`
        (`/Engine/EditorBlueprintResources/StandardMacros.DoOnce` true :!label _label
          (:`Completed`
            (set `self.startTouchLoc` _returnvalue))))
      (:`then_1`
        (`/Game/Maps/Overworld_UI.dragScreen` (`self.GUI`) (- _returnvalue (`self.startTouchLoc`)))))
    (else
      (`/Game/Maps/Overworld_UI.finishDrag` (`self.GUI`))
      (goto _label :!via `Reset`))))

(fn `initUI`
  (bind _returnvalue (`|CreateWidget` "/Game/Maps/Overworld_UI.Overworld_UI_C" self))
  (bind _output_get (set `self.GUI` _returnvalue))
  (`UserWidget.AddToPlayerScreen` _output_get 0))

(fn `moveCamera`
  (params (drag :type "Vector2D Structure"))
  (bind (_x _y) (`KismetMathLibrary.BreakVector2D` drag))
  (bind _viewcontroller (`/Game/Maps/Overworld_SPRITE_BP.ViewController` (`self.spriteViewer`)))
  (`SceneComponent.K2_SetRelativeLocation` _viewcontroller (`KismetMathLibrary.MakeVector` _x (.y (`SceneComponent.RelativeLocation` _viewcontroller)) _y) false false))

(fn `UserConstructionScript`)