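; Actor for a garden creature (Figment) that roams, eats food to gain stats and can "spec up" into another form.
; It builds its mesh and materials from a FigmentInfo struct, and a tap triggers focus through GameController.
; Tick shrinks held food until eaten and drifts the actor toward random GardenHandler locations.
; Food heals and adds stat points; level-ups award DNA, which spec-up spends, with changes saved to GameManager.
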(event `self.ReceiveBeginPlay`
  (`self.initFigment`)
  (`self.initCamera`))

(event `self.ReceiveTick`
  (params (DeltaSeconds :type "Float (single-precision)"))
  (`|ExecutionSequence`
    (:`then_0`
      (`self.eatingLogic`)
      (`self.waitToRoam`))
    (:`then_1`
      (`self.roamingLogic` DeltaSeconds))))

(event `self.ReceiveActorOnInputTouchBegin`
  (params (FingerIndex :type "ETouchIndex Enum" :default "Touch1"))
  (bind _asgame_controller (cast `/Game/System/Control/GameController` (`GameplayStatics.GetPlayerController` 0)))
  (if (not (`/Game/System/Control/GameController.figmentFocused?` _asgame_controller))
    (`/Game/System/Control/GameController.triggerFigmentFocus` _asgame_controller self)))

(event `self.FigmentMesh.OnInputTouchEnter`
  (params (FingerIndex :type "ETouchIndex Enum" :default "Touch1") (TouchedComponent :type "PrimitiveComponent Object Reference")))

(event `self.FigmentMesh.OnInputTouchLeave`
  (params (FingerIndex :type "ETouchIndex Enum" :default "Touch1") (TouchedComponent :type "PrimitiveComponent Object Reference")))

(event `self.FigmentSelectionRadius.OnInputTouchEnter`
  (params (FingerIndex :type "ETouchIndex Enum" :default "Touch1") (TouchedComponent :type "PrimitiveComponent Object Reference"))
  (set `self.hoveredOver` true))

(event `self.FigmentSelectionRadius.OnInputTouchLeave`
  (params (FingerIndex :type "ETouchIndex Enum" :default "Touch1") (TouchedComponent :type "PrimitiveComponent Object Reference"))
  (`KismetSystemLibrary.Delay` 0.1)
  (set `self.hoveredOver` false))

(fn `addHappiness`
  (returns (happinessOut :type "Float (double-precision)"))
  (locals (happiness :type "Float (double-precision)"))
  (bind _returnvalue (+ (`BlueprintMapLibrary.Map_Find` (`.FloatAttributes_106_99E6C55B4EBF4A7691CE25B72230BECF` (break `/Game/System/Types/Structs/Figment_STRUCT` (`self.figmentInfo`))) "Happiness") 0.1))
  (set `local.happiness` _returnvalue)
  (if (> _returnvalue 2.0)
    (set `local.happiness` 2.0))
  (return (`local.happiness`)))

(fn `addStatPoints`
  (params (StatToIncrease :type String) (PointsToGain :type Integer))
  (locals (statGained :type String) (statPtsKey :type String) (newPtAmt :type Integer) (ptsGained :type Integer) (statsMap :type "Map of String to Integer"))
  (bind ((`CompendiumNo_112_71757C554065C0862E4A4EB5C6BAE7CC` _compendiumno) (`Stats_10_D44B223F435FA506CFE9549967B720C4` _stats)) (break `/Game/System/Types/Structs/Figment_STRUCT` (`self.figmentInfo`)))
  (bind _returnvalue (`KismetStringLibrary.Concat_StrStr` (`local.statGained`) "Pts"))
  (bind _returnvalue_2 (`KismetStringLibrary.Concat_StrStr` (`local.statGained`) "Lvl"))
  (set `local.statsMap` (`.Stats_10_D44B223F435FA506CFE9549967B720C4` (break `/Game/System/Types/Structs/Figment_STRUCT` (`self.figmentInfo`))))
  (set `local.ptsGained` PointsToGain)
  (set `local.statGained` StatToIncrease)
  (set `local.statPtsKey` _returnvalue)
  (set `local.newPtAmt` (+ (`BlueprintMapLibrary.Map_Find` (`.Stats_10_D44B223F435FA506CFE9549967B720C4` (break `/Game/System/Types/Structs/Figment_STRUCT` (`self.figmentInfo`))) _returnvalue) (`local.ptsGained`)))
  (if (>= (`local.newPtAmt`) 5)
    (`BlueprintMapLibrary.Map_Add` _stats (`local.statPtsKey`) (mod (`local.newPtAmt`) 5))
    (`BlueprintMapLibrary.Map_Add` _stats _returnvalue_2 (+ (`BlueprintMapLibrary.Map_Find` _stats _returnvalue_2) 1))
    (`self.collectDNA`)
    (`self.tryHPBoost` (`local.statGained`))
    (else
      (`BlueprintMapLibrary.Map_Add` (`.Stats_10_D44B223F435FA506CFE9549967B720C4` (break `/Game/System/Types/Structs/Figment_STRUCT` (`self.figmentInfo`))) (`local.statPtsKey`) (`local.newPtAmt`))))
  (bind _asgame_controller (cast `/Game/System/Control/GameController` (`GameplayStatics.GetPlayerController` 0)))
  (bind _happinessout (`self.addHappiness`))
  (`BlueprintMapLibrary.Map_Add` (`.FloatAttributes_106_99E6C55B4EBF4A7691CE25B72230BECF` (break `/Game/System/Types/Structs/Figment_STRUCT` (`self.figmentInfo`))) "Happiness" _happinessout)
  (`/Game/System/Flow/GameManager.UpdateFigmentInGarden` (`/Game/System/Flow/GardenHandler.GameManager` (`self.GardenHandler`)) (`self.figmentInfo`))
  (`/Game/Maps/UI/FigmentFocus_UI.updateStats` (`/Game/System/Control/GameController.FigmentFocusGUI` _asgame_controller) (`self.figmentInfo`) (`local.statGained`)))

(fn `beginSpecUp`
  (bind ((`Name_6_628E0B664D16A10215B2DC96C335361B` _name) (`CompendiumNo_112_71757C554065C0862E4A4EB5C6BAE7CC` _compendiumno) (`Stats_10_D44B223F435FA506CFE9549967B720C4` _stats) (`Grades_44_0FD2490D485E2BAFA9F4FCA90852C89B` _grades) (`Texture_82_D64F4E0A49C23E408301C48BE5444740` _texture) (`FigmentID_97_FE0DBB1D4B5B90AADC680AB86EB54250` _figmentid) (`DNAType_56_05912AAD423657CC93CAF89197601018` _dnatype) (`PotentialSpecUps_65_A69E4C234627788FD5DC389BEB900C4B` _potentialspecups) (`SpecUpMultipliers_73_665A2B254917CBE04DD096ADA560D0E4` _specupmultipliers) (`OnJourney?_76_D97E1AF54E9ED850F7DE8EA585ECC4CD` _onjourney_) (`LocatedInGarden_79_2ED7C43C48B8BF5B1EDB5CABCA2125DA` _locatedingarden)) (break `/Game/System/Types/Structs/Figment_STRUCT` (`self.figmentInfo`)))
  (bind _asgame_manager (cast `/Game/System/Flow/GameManager` (`GameplayStatics.GetGameInstance`)))
  (`/Game/System/Flow/GameManager.RemoveDNA` _asgame_manager _dnatype 30)
  (bind _result (`self.findSpecUpResult`))
  (bind _output_get (set `self.figmentInfo` _result))
  (`self.resetFigment`)
  (`/Game/System/Flow/GameManager.AddFigmentToGarden` _asgame_manager _locatedingarden _output_get))

(fn `calcNextRoamLocation`
  (bind _location (`/Game/System/Flow/GardenHandler.Generate Random Location` (`self.GardenHandler`) true))
  (set `self.roamLocation` _location)
  (`self.K2_SetActorRotation` (`KismetMathLibrary.MakeRotator` (.roll (`KismetMathLibrary.FindLookAtRotation` (`self.K2_GetActorLocation`) (`self.roamLocation`))) (.pitch (`KismetMathLibrary.FindLookAtRotation` (`self.K2_GetActorLocation`) (`self.roamLocation`))) (- (.yaw (`KismetMathLibrary.FindLookAtRotation` (`self.K2_GetActorLocation`) (`self.roamLocation`))) 90.0)))
  (set `self.roaming` true))

(fn `collectDNA`
  (bind _asgame_manager (cast `/Game/System/Flow/GameManager` (`GameplayStatics.GetGameInstance`)))
  (`/Game/System/Flow/GameManager.AddDNA` _asgame_manager (`.DNAType_56_05912AAD423657CC93CAF89197601018` (break `/Game/System/Types/Structs/Figment_STRUCT` (`self.figmentInfo`))) 5)
  (bind _asgame_controller (cast `/Game/System/Control/GameController` (`GameplayStatics.GetPlayerController` 0)))
  (`/Game/Maps/UI/FigmentFocus_UI.updateDNA` (`/Game/System/Control/GameController.FigmentFocusGUI` _asgame_controller)))

(fn `eatFood`
  (params (food :type "/Game/System/Types/Structs/Item_STRUCT Structure"))
  (locals (statGained :type String))
  (bind ((`AffectType_20_115D1CD9441DC3CCCC8A3B8A936EC04B` _affecttype) (`AffectAmt_11_04270E5845317F0DDC91E5A77DAB98AB` _affectamt) (`HealAmt_59_626299C04AFD4C76EB2F52AC6A66710D` _healamt)) (break `/Game/System/Types/Structs/Item_STRUCT` food))
  (`|ExecutionSequence`
    (:`then_0`
      (switch `/Game/System/Types/Enums/AffectTypes` _affecttype
        (:`NewEnumerator0`
          (set `local.statGained` "Stamina"))
        (:`NewEnumerator2`
          (set `local.statGained` "Attack"))
        (:`NewEnumerator6`
          (set `local.statGained` "Defense"))
        (:`NewEnumerator3`
          (set `local.statGained` "EnergyAttack"))
        (:`NewEnumerator4`
          (set `local.statGained` "Agility"))))
    (:`then_1`
      (`self.recoverHealth` _healamt)
      (`self.addStatPoints` (`local.statGained`) (`KismetMathLibrary.FTrunc` _affectamt))
      (cast `/Game/System/Control/GameController` (`GameplayStatics.GetPlayerController` 0))
      (`self.startEating` food))))

(fn `eatingLogic`
  (if (`self.isEating`)
    (if (== (`SceneComponent.K2_GetComponentScale` (`self.heldItem`)) (0.0 0.0 0.0) :`ErrorTolerance` 0.05)
      (`self.finishEating`)
      (else
        (`self.takeBite`)))))

(fn `findSpecUpResult`
  (returns (result :type "/Game/System/Types/Structs/Figment_STRUCT Structure"))
  (bind ((`Name_6_628E0B664D16A10215B2DC96C335361B` _name) (`CompendiumNo_112_71757C554065C0862E4A4EB5C6BAE7CC` _compendiumno) (`Stats_10_D44B223F435FA506CFE9549967B720C4` _stats) (`Grades_44_0FD2490D485E2BAFA9F4FCA90852C89B` _grades) (`Texture_82_D64F4E0A49C23E408301C48BE5444740` _texture) (`FigmentID_97_FE0DBB1D4B5B90AADC680AB86EB54250` _figmentid) (`DNAType_56_05912AAD423657CC93CAF89197601018` _dnatype) (`PotentialSpecUps_65_A69E4C234627788FD5DC389BEB900C4B` _potentialspecups) (`SpecUpMultipliers_73_665A2B254917CBE04DD096ADA560D0E4` _specupmultipliers) (`OnJourney?_76_D97E1AF54E9ED850F7DE8EA585ECC4CD` _onjourney_) (`LocatedInGarden_79_2ED7C43C48B8BF5B1EDB5CABCA2125DA` _locatedingarden)) (break `/Game/System/Types/Structs/Figment_STRUCT` (`self.figmentInfo`)))
  (bind _keys (`BlueprintMapLibrary.Map_Keys` _potentialspecups))
  (bind _asgame_manager (cast `/Game/System/Flow/GameManager` (`GameplayStatics.GetGameInstance`)))
  (bind _figmentout (`/Game/System/Flow/GameManager.LookupFigmentFromTable` _asgame_manager (`|GetArrayItem` _keys)))
  (bind _structout (setmembers `/Game/System/Types/Structs/Figment_STRUCT` :`StructRef` _figmentout :`Stats` _stats :`Grades` _grades :`LocatedInGarden` _locatedingarden))
  (return _structout))

(fn `finishEating`
  (bind _helditem (`self.heldItem`))
  (setmembers `/Game/System/Types/Structs/Figment_STRUCT` :`StructRef` (`self.figmentInfo`) :`AnimState` "NewEnumerator0")
  (`SceneComponent.SetVisibility` _helditem false false)
  (`SceneComponent.SetWorldScale3D` _helditem (`self.initialItemScale`))
  (set `self.isEating` false))

(fn `focusOnFigment`)

(fn `getStat`
  (params (Stat :type String) (Type :type String))
  (returns (StatOut :type Integer))
  (return (`BlueprintMapLibrary.Map_Find` (`.Stats_10_D44B223F435FA506CFE9549967B720C4` (break `/Game/System/Types/Structs/Figment_STRUCT` (`self.figmentInfo`))) (`KismetStringLibrary.Concat_StrStr` Stat Type))))

(fn `initCamera`
  (set `SpringArmComponent.TargetArmLength` (* (`BlueprintMapLibrary.Map_Find` (`.FloatAttributes_106_99E6C55B4EBF4A7691CE25B72230BECF` (break `/Game/System/Types/Structs/Figment_STRUCT` (`self.figmentInfo`))) "CameraScale") 227.0) (`self.SpringArm`)))

(fn `initFigment`
  (bind _figmentmesh (`self.FigmentMesh`))
  (bind ((`Name_6_628E0B664D16A10215B2DC96C335361B` _name) (`CompendiumNo_112_71757C554065C0862E4A4EB5C6BAE7CC` _compendiumno) (`Grades_44_0FD2490D485E2BAFA9F4FCA90852C89B` _grades) (`Mesh_3_9607DBC34BC2F5BB7ED7F1BC401DC814` _mesh) (`AnimBlueprint_28_33CACA1A429DD8ACEA0C43957705C9F4` _animblueprint) (`Skin_22_C27CA512400D9FE23B7B4E9F6ABAB8A4` _skin) (`Texture_82_D64F4E0A49C23E408301C48BE5444740` _texture)) (break `/Game/System/Types/Structs/Figment_STRUCT` (`self.figmentInfo`)))
  (`|ExecutionSequence`
    (:`then_0`
      (`SkinnedMeshComponent.SetSkinnedAssetAndUpdate` _figmentmesh _mesh true)
      (`SkeletalMeshComponent.SetAnimInstanceClass` _figmentmesh _animblueprint)
      (setmembers `/Game/System/Types/Structs/Figment_STRUCT` :`StructRef` (`self.figmentInfo`) :`AnimState` "NewEnumerator0")
      (`SceneComponent.K2_SetWorldLocation` (`self.FigmentSelectionRadius`) (`SceneComponent.GetSocketLocation` (`self.FigmentMesh`) "feedRadius") false false)
      (bind _asgarden_handler (cast `/Game/System/Flow/GardenHandler` (`GameplayStatics.GetGameMode`)))
      (set `self.GardenHandler` _asgarden_handler))
    (:`then_1`
      (bind _returnvalue (`KismetMaterialLibrary.CreateDynamicMaterialInstance` _skin))
      (`MaterialInstanceDynamic.SetTextureParameterValue` _returnvalue "Texture" (`BlueprintMapLibrary.Map_Find` _texture "Body"))
      (`PrimitiveComponent.SetMaterialByName` (`self.FigmentMesh`) "Body" _returnvalue))
    (:`then_2`
      (bind _returnvalue_2 (`KismetMaterialLibrary.CreateDynamicMaterialInstance` _skin))
      (`MaterialInstanceDynamic.SetTextureParameterValue` _returnvalue_2 "Texture" (`BlueprintMapLibrary.Map_Find` _texture "Face"))
      (`PrimitiveComponent.SetMaterialByName` (`self.FigmentMesh`) "Face" _returnvalue_2))))

(fn `initHeldItem`
  (params (item :type "/Game/System/Types/Structs/Item_STRUCT Structure"))
  (bind ((`GrabBagType_37_586E0B4E4B85A2AEF6F90FBFD6959350` _grabbagtype) (`GenericAttributes_55_D6722D7841E26365D9109685356AAEA3` _genericattributes) (`GrabBagTable_43_3DD7368D493DC0ED7BE3B4A88A286D47` _grabbagtable) (`EggHatchTable_53_0F1B2C844CBDAE338F1ECC9852AAEC28` _egghatchtable) (`HealAmt_59_626299C04AFD4C76EB2F52AC6A66710D` _healamt) (`Mesh_16_34F2F29B497BD98F277B64AA5036BAE8` _mesh) (`Skin_28_3B90DAAE4AF528F471C5FBBA8DFC83DB` _skin) (`Texture_29_0E1DA06B4C082667184D7F8593243CE8` _texture)) (break `/Game/System/Types/Structs/Item_STRUCT` item))
  (bind _helditem (`self.heldItem`))
  (set `self.initialItemScale` (`SceneComponent.K2_GetComponentScale` (`self.heldItem`)))
  (`StaticMeshComponent.SetStaticMesh` _helditem _mesh)
  (`SceneComponent.SetVisibility` _helditem true false)
  (bind _returnvalue (`KismetMaterialLibrary.CreateDynamicMaterialInstance` _skin))
  (`MaterialInstanceDynamic.SetTextureParameterValue` _returnvalue "Texture" _texture)
  (`PrimitiveComponent.SetMaterial` (`self.heldItem`) 0 _returnvalue))

(fn `recoverHealth`
  (params (healthToRecover :type Integer))
  (bind _figmentinfo (`self.figmentInfo`))
  (bind (_name _compendiumno _stats) (break `/Game/System/Types/Structs/Figment_STRUCT` _figmentinfo))
  (bind _returnvalue (+ (`BlueprintMapLibrary.Map_Find` _stats "CurrentStamina") healthToRecover))
  (bind _rawpower (`/Game/System/Functions/UniversalFunctions.calculateRawStatPower` "Stamina" _figmentinfo))
  (if (> _returnvalue _rawpower)
    (`BlueprintMapLibrary.Map_Add` _stats "CurrentStamina" _rawpower)
    (else
      (`BlueprintMapLibrary.Map_Add` _stats "CurrentStamina" _returnvalue))))

(fn `resetFigment`
  (`self.initFigment`)
  (bind _asgame_controller (cast `/Game/System/Control/GameController` (`GameplayStatics.GetPlayerController` 0)))
  (`/Game/Maps/UI/FigmentFocus_UI.initStats` (`/Game/System/Control/GameController.FigmentFocusGUI` _asgame_controller)))

(fn `roamingLogic`
  (params (delta :type "Float (double-precision)"))
  (locals (xVal :type "Float (double-precision)") (yVal :type "Float (double-precision)"))
  (bind _returnvalue (`self.K2_GetActorLocation`))
  (bind _roamlocation (`self.roamLocation`))
  (if (and (`self.roaming`) (`self.canRoam`))
    (`self.K2_SetActorLocation` (`KismetMathLibrary.VInterpTo` _returnvalue _roamlocation delta 0.2))
    (if (or (< (`KismetMathLibrary.Vector_Distance` _returnvalue _roamlocation) 300.0) (> (`KismetArrayLibrary.Array_Length` (`PrimitiveComponent.GetOverlappingActors` (`self.ObstacleDetector`) "/Game/Maps/GenericTools/Obstacle.Obstacle_C")) 0))
      (set `self.roaming` false))))

(fn `startEating`
  (params (item :type "/Game/System/Types/Structs/Item_STRUCT Structure"))
  (set `self.isEating` true)
  (`self.initHeldItem` item)
  (setmembers `/Game/System/Types/Structs/Figment_STRUCT` :`StructRef` (`self.figmentInfo`) :`AnimState` "NewEnumerator3"))

(fn `takeBite`
  (bind _helditem (`self.heldItem`))
  (`SceneComponent.SetWorldScale3D` _helditem (- (`SceneComponent.K2_GetComponentScale` _helditem) 0.001))
  (`SceneComponent.K2_SetWorldLocation` (`self.heldItem`) (`SceneComponent.GetSocketLocation` (`self.FigmentMesh`) "heldItem") false false))

(fn `takeItem`
  (params (item :type "/Game/System/Types/Structs/Item_STRUCT Structure"))
  (`|ExecutionSequence`
    (:`then_0`
      (switch `/Game/System/Types/Enums/ItemTypes` (`.Type_5_79367EC34A82EDDA80D3F188256374E0` (break `/Game/System/Types/Structs/Item_STRUCT` item))
        (:`NewEnumerator0`
          (`self.eatFood` item))))
    (:`then_1`
      (bind _asgame_manager (cast `/Game/System/Flow/GameManager` (`GameplayStatics.GetGameInstance`)))
      (`/Game/System/Flow/GameManager.UpdateFigmentInGarden` _asgame_manager (`self.figmentInfo`)))))

(fn `tryHPBoost`
  (params (Stat :type String))
  (bind ((`CompendiumNo_112_71757C554065C0862E4A4EB5C6BAE7CC` _compendiumno) (`Stats_10_D44B223F435FA506CFE9549967B720C4` _stats) (`Grades_44_0FD2490D485E2BAFA9F4FCA90852C89B` _grades) (`Texture_82_D64F4E0A49C23E408301C48BE5444740` _texture) (`FigmentID_97_FE0DBB1D4B5B90AADC680AB86EB54250` _figmentid) (`SpecUpMultipliers_73_665A2B254917CBE04DD096ADA560D0E4` _specupmultipliers)) (break `/Game/System/Types/Structs/Figment_STRUCT` (`self.figmentInfo`)))
  (bind _value (`BlueprintMapLibrary.Map_Find` _stats "StaminaLvl"))
  (bind _value_2 (`BlueprintMapLibrary.Map_Find` _specupmultipliers "Stamina"))
  (if (`KismetStringLibrary.EqualEqual_StrStr` Stat "Stamina")
    (bind _gradevalue (`/Game/System/Functions/UniversalFunctions.getGradeValue` (`BlueprintMapLibrary.Map_Find` _grades "Stamina")))
    (`BlueprintMapLibrary.Map_Add` _stats "CurrentStamina" (+ (`BlueprintMapLibrary.Map_Find` _stats "CurrentStamina") (`KismetMathLibrary.Round` (- (* _gradevalue (* _value _value_2)) (* _gradevalue (* (- _value 1) _value_2))))))))

(fn `UserConstructionScript`)

(fn `waitToRoam`
  (if (and (not (`self.roaming`)) (`self.canRoam`))
    (if (== (`KismetMathLibrary.RandomInteger` 500) (`KismetMathLibrary.RandomInteger` 500))
      (`self.calcNextRoamLocation`))))

(fn `willFigmentAcceptItem`
  (params (item :type "/Game/System/Types/Structs/Item_STRUCT Structure"))
  (returns (willAccept :type Boolean))
  (bind ((`Type_5_79367EC34A82EDDA80D3F188256374E0` _type) (`GrabBagType_37_586E0B4E4B85A2AEF6F90FBFD6959350` _grabbagtype) (`GenericAttributes_55_D6722D7841E26365D9109685356AAEA3` _genericattributes) (`GrabBagTable_43_3DD7368D493DC0ED7BE3B4A88A286D47` _grabbagtable) (`EggHatchTable_53_0F1B2C844CBDAE338F1ECC9852AAEC28` _egghatchtable) (`HealAmt_59_626299C04AFD4C76EB2F52AC6A66710D` _healamt) (`Fillingness_34_3A01214A4EBB21EF88409D8D8EB8A1F9` _fillingness)) (break `/Game/System/Types/Structs/Item_STRUCT` item))
  (bind ((`CompendiumNo_112_71757C554065C0862E4A4EB5C6BAE7CC` _compendiumno) (`Stats_10_D44B223F435FA506CFE9549967B720C4` _stats)) (break `/Game/System/Types/Structs/Figment_STRUCT` (`self.figmentInfo`)))
  (switch `/Game/System/Types/Enums/ItemTypes` _type
    (:`NewEnumerator0`
      (if (not (`self.isEating`))
        (if (> (`BlueprintMapLibrary.Map_Find` _stats "StomachCapacity") (+ (`BlueprintMapLibrary.Map_Find` _stats "StomachFullness") _fillingness))
          (return true)
          (else
            (`/Game/System/Functions/UniversalFunctions.ReportMessage` "Not hungry" "NewEnumerator2")))
        (else
          (`/Game/System/Functions/UniversalFunctions.ReportMessage` "This figment is still eating" "NewEnumerator2")
          (return false))))))