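; Figment character for a turn-based, grid-based mystery dungeon, either player-controlled or moved randomly by AI.
; InitFigment builds its mesh, animation and body/face materials from the FigmentInfo struct.
; Eight-way input turns the mesh and steps onto traversable handler tiles, with Tick interpolating position using a fixed delta.
; FinishTurn collects tile items and releases the turn; tapping a controlled Figment opens the main menu.
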(event `self.ReceiveBeginPlay`
  (`self.initFigment`))

(event `self.ReceiveTick`
  (params (DeltaSeconds :type "Float (single-precision)"))
  (if (`self.traveling`)
    (`self.tickOntoPanel` DeltaSeconds)))

(event `self.ReceiveActorOnInputTouchBegin`
  (params (FingerIndex :type "ETouchIndex Enum" :default "Touch1")))

(event `self.FigmentSelectionRadius.OnInputTouchBegin`
  (params (FingerIndex :type "ETouchIndex Enum" :default "Touch1") (TouchedComponent :type "PrimitiveComponent Object Reference"))
  (if (`self.controlled`)
    (set `self.touched` true)))

(event `self.FigmentSelectionRadius.OnInputTouchEnd`
  (params (FingerIndex :type "ETouchIndex Enum" :default "Touch1") (TouchedComponent :type "PrimitiveComponent Object Reference"))
  (if (`self.touched`)
    (set `self.touched` false)
    (bind _asmystery_dungeon_controller (cast `/Game/System/Control/MysteryDungeonController` (`GameplayStatics.GetPlayerController` 0)))
    (`/Game/Maps/MysteryDungeon/MysteryDungeonUI.toggleMainMenu` (`/Game/System/Control/MysteryDungeonController.MDUI` _asmystery_dungeon_controller) true)))

(fn `[AI]CalculateNextAction`
  (bind _randomdirection (`/Game/System/Functions/UniversalFunctions.makeRandomDirection`))
  (`self.takeMovementInput` _randomdirection)
  (`self.finishTurn`))

(fn `finishTurn`
  (bind _output (`|GetArrayItem` (`/Game/System/Flow/MysteryDungeonHandler.floorTiles` (`self.MDHandler`)) (`self.currentLocation`)))
  (`|ExecutionSequence`
    (:`then_0`
      (if (`/Game/Maps/MysteryDungeon/Blocks/Block.isItemOnBlock?` _output)
        (bind _itemtaken (`/Game/Maps/MysteryDungeon/Blocks/Block.removeItemFromBlock` _output))
        (if (`self.controlled`)
          (bind _asgame_manager (cast `/Game/System/Flow/Universal/GameManager` (`GameplayStatics.GetGameInstance`)))
          (`/Game/System/Flow/Universal/GameManager.AddItemToInventory` _asgame_manager _itemtaken 1)
          (else
            (`KismetArrayLibrary.Array_Add` (`self.figmentInventory`) _itemtaken)))))
    (:`then_1`
      (set `self.takingTurn` false)
      (set `/Game/System/Flow/MysteryDungeonHandler.currentFigmentTakingTurn` false (`self.MDHandler`)))))

(fn `initFigment`
  (bind _figmentmesh (`self.FigmentMesh`))
  (bind ((`Mesh_3_9607DBC34BC2F5BB7ED7F1BC401DC814` _mesh) (`AnimBlueprint_28_33CACA1A429DD8ACEA0C43957705C9F4` _animblueprint) (`AnimState_36_2BB6F3334D56C2EE90142595588FDDB7` _animstate) (`PotentialSpecUps_65_A69E4C234627788FD5DC389BEB900C4B` _potentialspecups) (`TextureAttributes_127_D64F4E0A49C23E408301C48BE5444740` _textureattributes) (`StringAttributes_93_4E8689CE402656D158BBD0939F8E4CD3` _stringattributes) (`IntegerAttributes_114_7F9E46E04026B577C97B00BEB50E067E` _integerattributes) (`FloatAttributes_106_99E6C55B4EBF4A7691CE25B72230BECF` _floatattributes) (`LastInteractedWith_109_AE1EE488475DF898429B83B6238FBEDB` _lastinteractedwith) (`EquippableChips_119_242DF7F749F3D359EE0E62AF231E76B6` _equippablechips) (`EquippedChips_122_11420D3D45FD81EAEFD49093864A350B` _equippedchips) (`Skin_22_C27CA512400D9FE23B7B4E9F6ABAB8A4` _skin) (`Texture_82_D64F4E0A49C23E408301C48BE5444740` _texture)) (break `/Game/System/Types/Structs/Figment_STRUCT` (`self.figmentInfo`)))
  (`|ExecutionSequence`
    (:`then_0`
      (`SkinnedMeshComponent.SetSkinnedAssetAndUpdate` _figmentmesh _mesh true)
      (`SkeletalMeshComponent.SetAnimInstanceClass` _figmentmesh _animblueprint)
      (setmembers `/Game/System/Types/Structs/Figment_STRUCT` :`StructRef` (`self.figmentInfo`) :`AnimState` "NewEnumerator0")
      (bind _asmystery_dungeon_handler (cast `/Game/System/Flow/MysteryDungeonHandler` (`GameplayStatics.GetGameMode`)))
      (set `self.MDHandler` _asmystery_dungeon_handler))
    (:`then_1`
      (bind _returnvalue (`KismetMaterialLibrary.CreateDynamicMaterialInstance` _skin))
      (`MaterialInstanceDynamic.SetTextureParameterValue` _returnvalue "Texture" (`BlueprintMapLibrary.Map_Find` _texture "Body"))
      (`PrimitiveComponent.SetMaterialByName` (`self.FigmentMesh`) "Body" _returnvalue))
    (:`then_2`
      (bind _returnvalue_2 (`KismetMaterialLibrary.CreateDynamicMaterialInstance` _skin))
      (`MaterialInstanceDynamic.SetTextureParameterValue` _returnvalue_2 "Texture" (`BlueprintMapLibrary.Map_Find` _texture "Face"))
      (`PrimitiveComponent.SetMaterialByName` (`self.FigmentMesh`) "Face" _returnvalue_2))))

(fn `PlanStep`
  (params (xDir :type Integer) (yDir :type Integer) (turnDir :type "Float (double-precision)"))
  (locals (xDirection :type Integer) (yDirection :type Integer) (boundarySize :type Integer) (widthOfFloor :type Integer) (xIncrement :type Integer))
  (bind _mdhandler (`self.MDHandler`))
  (set `local.boundarySize` (`/Game/System/Flow/MysteryDungeonHandler.OutOfBoundsSize` _mdhandler))
  (set `local.widthOfFloor` (`/Game/System/Flow/MysteryDungeonHandler.floorWidth` _mdhandler))
  (set `local.xDirection` xDir)
  (set `local.yDirection` yDir)
  (`self.turn` turnDir)
  (if (`/Game/Maps/MysteryDungeon/Blocks/Block.isTraversable` (`|GetArrayItem` (`/Game/System/Flow/MysteryDungeonHandler.floorTiles` (`self.MDHandler`)) (+ (+ (`self.currentLocation`) (* (`local.widthOfFloor`) (`local.yDirection`))) (`local.xDirection`))))
    (bind _output_get (set `self.currentLocation` (+ (+ (`self.currentLocation`) (* (`local.widthOfFloor`) (`local.yDirection`))) (`local.xDirection`))))
    (`self.tryStepOntoPanel` (`|GetArrayItem` (`/Game/System/Flow/MysteryDungeonHandler.floorTiles` (`self.MDHandler`)) _output_get) _output_get)))

(fn `stopMoving`
  (set `self.traveling` false)
  (setmembers `/Game/System/Types/Structs/Figment_STRUCT` :`StructRef` (`self.figmentInfo`) :`AnimState` "NewEnumerator0")
  (`self.K2_SetActorLocation` (`self.targetLocation`))
  (set `self.touched` true))

(fn `takeMovementInput`
  (params (InputDir :type "/Game/System/Types/Enums/MovementTypes Enum" :default "NewEnumerator8"))
  (locals (controlledFigment :type "/Game/Actors/Figments/MD_Figment_BP Object Reference"))
  (switch `/Game/System/Types/Enums/MovementTypes` InputDir
    (:`NewEnumerator0`
      (`self.PlanStep` 0 -1 180.0)
      (`self.finishTurn` :!label _label))
    (:`NewEnumerator1`
      (`self.PlanStep` 0 1)
      (goto _label))
    (:`NewEnumerator2`
      (`self.PlanStep` -1 0 90.0)
      (goto _label))
    (:`NewEnumerator3`
      (`self.PlanStep` 1 0 -90.0)
      (`self.finishTurn` :!label _label_2))
    (:`NewEnumerator4`
      (`self.PlanStep` -1 -1 135.0)
      (goto _label_2))
    (:`NewEnumerator5`
      (`self.PlanStep` 1 -1 225.0)
      (`self.finishTurn` :!label _label_3))
    (:`NewEnumerator6`
      (`self.PlanStep` -1 1 45.0)
      (goto _label_3))
    (:`NewEnumerator7`
      (`self.PlanStep` 1 1 -45.0)
      (goto _label_3))))

(fn `tickOntoPanel`
  (params (delta :type "Float (double-precision)"))
  (`self.K2_SetActorLocation` (`KismetMathLibrary.VInterpTo_Constant` (`self.K2_GetActorLocation`) (`self.targetLocation`) 0.35 10.0))
  (if (== (`self.K2_GetActorLocation`) (`self.targetLocation`) :`ErrorTolerance` 0.01)
    (set `self.traveling` false)
    (setmembers `/Game/System/Types/Structs/Figment_STRUCT` :`StructRef` (`self.figmentInfo`) :`AnimState` "NewEnumerator0")
    (`self.K2_SetActorLocation` (`self.targetLocation`))))

(fn `tryStepOntoPanel`
  (params (panelRef :type "/Game/Maps/MysteryDungeon/Blocks/Block Object Reference") (panelIndex :type Integer))
  (set `self.currentLocation` panelIndex)
  (set `self.targetLocation` (`SceneComponent.K2_GetComponentLocation` (`/Game/Maps/MysteryDungeon/Blocks/Block.FigmentStepLocation` panelRef)))
  (set `self.traveling` true)
  (setmembers `/Game/System/Types/Structs/Figment_STRUCT` :`StructRef` (`self.figmentInfo`) :`AnimState` "NewEnumerator6"))

(fn `turn`
  (params (ZTurn :type "Float (double-precision)"))
  (`SceneComponent.K2_SetWorldRotation` (`self.FigmentMesh`) (`KismetMathLibrary.MakeRotator` 0.0 0.0 ZTurn) false false))

(fn `UserConstructionScript`)