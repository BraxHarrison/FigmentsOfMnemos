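; Base Blueprint for a touchable Figment actor placed in the world.
; On BeginPlay it caches the FoM_MANAGER game instance, looks up its data by FigmentID and passes it to InitFigmentAppearance, which is empty here.
; Touching its InteractionRadius component asks the Player_PC controller to request that figment's info.
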(event `self.ReceiveBeginPlay`
  (`self.LinkReferences`)
  (`self.InitFigment`))

(event `self.InteractionRadius.OnInputTouchBegin`
  (params (FingerIndex :type "ETouchIndex Enum" :default "Touch1") (TouchedComponent :type "PrimitiveComponent Object Reference"))
  (bind _asplayer_pc (cast `/Game/Actors/Characters/Player/Base/Player_PC` (`GameplayStatics.GetPlayerController` 0)))
  (`/Game/Actors/Characters/Player/Base/Player_PC.requestFigmentInfo` _asplayer_pc self))

(fn `InitFigment`
  (locals (figmentInfo :type "/Game/Actors/Figments/Base/Figment_INFO Structure"))
  (bind _outfigment (`/Game/System/Flow/FoM_MANAGER.FindFigmentWithID` (`self.manager`) (`self.figmentID`)))
  (bind _output_get (set `local.figmentInfo` _outfigment))
  (`self.InitFigmentAppearance` _output_get))

(fn `InitFigmentAppearance`
  (params (FigmentRef :type "/Game/Actors/Figments/Base/Figment_INFO Structure")))

(fn `LinkReferences`
  (bind _asfo_m_manager (cast `/Game/System/Flow/FoM_MANAGER` (`GameplayStatics.GetGameInstance`)))
  (set `self.manager` _asfo_m_manager))

(fn `UserConstructionScript`)