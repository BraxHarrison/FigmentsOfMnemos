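; ControlledFigment_BP is a figment actor that builds its appearance at runtime from its FigmentInfo struct.
; On BeginPlay it prints a debug string, caches the GameManager game instance and, if that cast succeeds, initializes the figment.
; Initialization applies the skeletal mesh and anim class, sets the struct's AnimState, then creates separate dynamic skin materials for the Body and Face slots, textured via map lookups.
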(event `self.ReceiveBeginPlay`
  (`KismetSystemLibrary.PrintString` "PLEASE")
  (bind _asgame_manager (cast `/Game/System/Flow/Universal/GameManager` (`GameplayStatics.GetGameInstance`)))
  (set `self.GameManager` _asgame_manager)
  (`self.initFigmentInstance`))

(fn `initFigmentInstance`
  (bind _mesh (`self.Mesh`))
  (bind ((`Name_6_628E0B664D16A10215B2DC96C335361B` _name) (`CompendiumNo_112_71757C554065C0862E4A4EB5C6BAE7CC` _compendiumno) (`Grades_44_0FD2490D485E2BAFA9F4FCA90852C89B` _grades) (`Mesh_3_9607DBC34BC2F5BB7ED7F1BC401DC814` _mesh_2) (`AnimBlueprint_28_33CACA1A429DD8ACEA0C43957705C9F4` _animblueprint) (`Skin_22_C27CA512400D9FE23B7B4E9F6ABAB8A4` _skin) (`Texture_82_D64F4E0A49C23E408301C48BE5444740` _texture)) (break `/Game/System/Types/Structs/Figment_STRUCT` (`self.figmentInfo`)))
  (`|ExecutionSequence`
    (:`then_0`
      (`SkinnedMeshComponent.SetSkinnedAssetAndUpdate` _mesh _mesh_2 true)
      (`SkeletalMeshComponent.SetAnimInstanceClass` _mesh _animblueprint)
      (setmembers `/Game/System/Types/Structs/Figment_STRUCT` :`StructRef` (`self.figmentInfo`) :`AnimState` "NewEnumerator0"))
    (:`then_1`
      (bind _returnvalue (`KismetMaterialLibrary.CreateDynamicMaterialInstance` _skin))
      (`MaterialInstanceDynamic.SetTextureParameterValue` _returnvalue "Texture" (`BlueprintMapLibrary.Map_Find` _texture "Body"))
      (`PrimitiveComponent.SetMaterialByName` (`self.Mesh`) "Body" _returnvalue))
    (:`then_2`
      (bind _returnvalue_2 (`KismetMaterialLibrary.CreateDynamicMaterialInstance` _skin))
      (`MaterialInstanceDynamic.SetTextureParameterValue` _returnvalue_2 "Texture" (`BlueprintMapLibrary.Map_Find` _texture "Face"))
      (`PrimitiveComponent.SetMaterialByName` (`self.Mesh`) "Face" _returnvalue_2))))

(fn `UserConstructionScript`)