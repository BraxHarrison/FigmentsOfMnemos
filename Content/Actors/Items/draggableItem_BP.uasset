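; Draggable item actor that the player drags onto the garden's focused Figment to give it from the inventory.
; On BeginPlay it takes its mesh and textured dynamic material from ItemInfo.
; Touch starts a drag; Tick follows the deprojected mouse, checks whether the hovered Figment accepts the item and sets its anim state.
; Release either gives the item, updating inventory and widget before destroying the actor, or snaps it back.
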(event `self.ReceiveBeginPlay`
  (`self.initItem`))

(event `self.ReceiveTick`
  (params (DeltaSeconds :type "Float (single-precision)"))
  (`|ExecutionSequence`
    (:`then_0`
      (`self.updateDragLocation`))
    (:`then_1`
      (`self.checkOverlapping`))
    (:`then_2`
      (`self.checkMouseReleased`))))

(event `self.ReceiveActorOnInputTouchBegin`
  (params (FingerIndex :type "ETouchIndex Enum" :default "Touch1"))
  (set `self.isDragged` true)
  (`PrimitiveComponent.SetCollisionEnabled` (`self.StaticMesh`) "NoCollision"))

(fn `checkMouseReleased`
  (if (`self.isDragged`)
    (if (not (`/Game/System/Control/GameController.mouseDown` (`self.controller`)))
      (if (`self.ableToGive`)
        (`self.giveToFigment`)
        (else
          (`PrimitiveComponent.SetCollisionEnabled` (`self.StaticMesh`) "QueryOnly")))
      (set `self.isDragged` false))))

(fn `checkOverlapping`
  (bind _focusedfigment (`/Game/System/Flow/GardenHandler.focusedFigment` (`self.gameHandler`)))
  (if (`self.isDragged`)
    (if (`/Game/Actors/Figments/Figment_BP.hoveredOver` _focusedfigment)
      (bind _willaccept (`/Game/Actors/Figments/Figment_BP.willFigmentAcceptItem` _focusedfigment (`self.itemInfo`)))
      (if _willaccept
        (setmembers `/Game/System/Types/Structs/Figment_STRUCT` :`StructRef` (`/Game/Actors/Figments/Figment_BP.figmentInfo` (`/Game/System/Flow/GardenHandler.focusedFigment` (`self.gameHandler`))) :`AnimState` "NewEnumerator1")
        (set `self.ableToGive` true))
      (else
        (set `self.ableToGive` false)
        (setmembers `/Game/System/Types/Structs/Figment_STRUCT` :`StructRef` (`/Game/Actors/Figments/Figment_BP.figmentInfo` (`/Game/System/Flow/GardenHandler.focusedFigment` (`self.gameHandler`))) :`AnimState` "NewEnumerator0")))))

(fn `destroyItem`
  (`self.K2_DestroyActor`))

(fn `giveToFigment`
  (bind _iteminfo (`self.itemInfo`))
  (`/Game/Actors/Figments/Figment_BP.takeItem` (`/Game/System/Flow/GardenHandler.focusedFigment` (`/Game/System/Control/GameController.GardenHandler` (`self.controller`))) _iteminfo)
  (`/Game/System/Flow/GameManager.RemoveItemFromInventory` (`self.GameManager`) _iteminfo 1)
  (bind _structout (setmembers `/Game/System/Types/Structs/Item_STRUCT` :`StructRef` _iteminfo :`NumberInStack` (- (`.NumberInStack_23_C585ADF54AE6015C5281F787B6EA9678` (break `/Game/System/Types/Structs/Item_STRUCT` _iteminfo)) 1)))
  (`/Game/Maps/UI/Item_UI.updateItemInfo` (`self.widgetReference`) _structout)
  (`self.destroyItem`))

(fn `initItem`
  (bind ((`NumberInStack_23_C585ADF54AE6015C5281F787B6EA9678` _numberinstack) (`GrabBagType_37_586E0B4E4B85A2AEF6F90FBFD6959350` _grabbagtype) (`GenericAttributes_55_D6722D7841E26365D9109685356AAEA3` _genericattributes) (`GrabBagTable_43_3DD7368D493DC0ED7BE3B4A88A286D47` _grabbagtable) (`EggHatchTable_53_0F1B2C844CBDAE338F1ECC9852AAEC28` _egghatchtable) (`HealAmt_59_626299C04AFD4C76EB2F52AC6A66710D` _healamt) (`Fillingness_34_3A01214A4EBB21EF88409D8D8EB8A1F9` _fillingness) (`Mesh_16_34F2F29B497BD98F277B64AA5036BAE8` _mesh) (`Skin_28_3B90DAAE4AF528F471C5FBBA8DFC83DB` _skin) (`Texture_29_0E1DA06B4C082667184D7F8593243CE8` _texture)) (break `/Game/System/Types/Structs/Item_STRUCT` (`self.itemInfo`)))
  (`|ExecutionSequence`
    (:`then_0`
      (`StaticMeshComponent.SetStaticMesh` (`self.StaticMesh`) _mesh)
      (bind _asgame_controller (cast `/Game/System/Control/GameController` (`GameplayStatics.GetPlayerController` 0)))
      (set `self.controller` _asgame_controller)
      (set `self.initialPosition` (`self.K2_GetActorLocation`))
      (bind _asgame_manager (cast `/Game/System/Flow/GameManager` (`GameplayStatics.GetGameInstance`)))
      (set `self.GameManager` _asgame_manager))
    (:`then_1`
      (bind _returnvalue (`KismetMaterialLibrary.CreateDynamicMaterialInstance` _skin))
      (`MaterialInstanceDynamic.SetTextureParameterValue` _returnvalue "Texture" _texture)
      (`PrimitiveComponent.SetMaterial` (`self.StaticMesh`) 0 _returnvalue)
      (bind _asgarden_handler (cast `/Game/System/Flow/GardenHandler` (`GameplayStatics.GetGameMode`)))
      (set `self.gameHandler` _asgarden_handler))))

(fn `updateDragLocation`
  (bind (_worldlocation _worlddirection) (`PlayerController.DeprojectMousePositionToWorld` (`self.controller`)))
  (if (`self.isDragged`)
    (`self.K2_SetActorLocation` (`KismetMathLibrary.MakeVector` (.x (+ _worldlocation (* (* _worlddirection (- (/ (.y _worldlocation) (.y (`self.initialPosition`))) 20.0)) -1.0))) (.y (+ _worldlocation (* (* _worlddirection (- (/ (.y _worldlocation) (.y (`self.initialPosition`))) 20.0)) -1.0))) (.z (+ _worldlocation (* (* _worlddirection (- (/ (.y _worldlocation) (.y (`self.initialPosition`))) 20.0)) -1.0)))))
    (else
      (`self.K2_SetActorLocation` (`self.initialPosition`)))))

(fn `UserConstructionScript`)