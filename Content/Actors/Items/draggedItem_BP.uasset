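; Dragged item actor that displays an item's mesh and follows the mouse cursor in the garden.
; On BeginPlay, InitItem sets the static mesh from ItemInfo and caches the PC_Garden player controller.
; Each Tick deprojects the cursor and moves the root along that ray, scaling by the garden camera's offset Y over the ray's Y direction to hold the item at a consistent depth.
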(event `self.ReceiveBeginPlay`
  (`self.initItem`))

(event `self.ReceiveTick`
  (params (DeltaSeconds :type "Float (single-precision)"))
  (bind (_worldlocation _worlddirection) (`PlayerController.DeprojectMousePositionToWorld` (`self.playerController`)))
  (`WidgetLayoutLibrary.GetMousePositionOnViewport`)
  (`SceneComponent.K2_SetWorldLocation` (`self.DefaultSceneRoot`) (+ (`KismetMathLibrary.MakeVector` (.x _worldlocation) (.y _worldlocation) (.z _worldlocation)) (* (* _worlddirection (/ (+ (.y (`SceneComponent.K2_GetComponentLocation` (`/Game/Maps/Garden_BP.Camera` (`/Game/System/Flow/GM_Garden.instantiatedGarden` (`/Game/System/Control/PC_Garden.GameMode` (`self.playerController`)))))) -80.0) (.y _worlddirection))) -1.0)) false false))

(fn `initItem`
  (`StaticMeshComponent.SetStaticMesh` (`self.StaticMesh`) (`.Mesh_16_34F2F29B497BD98F277B64AA5036BAE8` (break `/Game/System/Types/Item_STRUCT` (`self.itemInfo`))))
  (bind _aspc_garden (cast `/Game/System/Control/PC_Garden` (`GameplayStatics.GetPlayerController` 0)))
  (set `self.playerController` _aspc_garden))

(fn `UserConstructionScript`)