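; Ingredient actor in the Workshop Blender map that falls while tumbling.
; On BeginPlay it sets its mesh from ItemInfo and applies a dynamic material built from the item's skin and texture.
; It then randomizes fall speed and spin rates and slightly jitters its horizontal position.
; Each Tick moves it down and adds the rotation by fixed per-frame amounts, without sweep or delta-time scaling.
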(event `self.ReceiveBeginPlay`
  (`self.initIngredient`)
  (`self.generateRandomValues`))

(event `self.ReceiveTick`
  (params (DeltaSeconds :type "Float (single-precision)"))
  (`self.moveDown`)
  (`self.randomRotation`))

(fn `generateRandomValues`
  (set `self.fallSpeed` (`KismetMathLibrary.RandomFloatInRange` 0.15 0.3))
  (set `self.xRot` (`KismetMathLibrary.RandomFloatInRange` 0.15 0.3))
  (set `self.yRot` (`KismetMathLibrary.RandomFloatInRange` -0.5 0.5))
  (set `self.zRot` (`KismetMathLibrary.RandomFloatInRange` -0.5 0.5))
  (`self.K2_SetActorLocation` (`KismetMathLibrary.MakeVector` (+ (.x (`self.K2_GetActorLocation`)) (`KismetMathLibrary.RandomFloatInRange` -2.0 2.0)) (+ (.y (`self.K2_GetActorLocation`)) (`KismetMathLibrary.RandomFloatInRange` -2.0 2.0)) (.z (`self.K2_GetActorLocation`)))))

(fn `initIngredient`
  (bind _ingredientmesh (`self.IngredientMesh`))
  (bind ((`Name_2_6239F61F4E3C209977966C8BB4803326` _name) (`Mesh_16_34F2F29B497BD98F277B64AA5036BAE8` _mesh) (`Skin_28_3B90DAAE4AF528F471C5FBBA8DFC83DB` _skin) (`Texture_29_0E1DA06B4C082667184D7F8593243CE8` _texture)) (break `/Game/System/Types/Structs/Item_STRUCT` (`self.itemInfo`)))
  (`StaticMeshComponent.SetStaticMesh` _ingredientmesh _mesh)
  (bind _returnvalue (`KismetMaterialLibrary.CreateDynamicMaterialInstance` _skin))
  (`MaterialInstanceDynamic.SetTextureParameterValue` _returnvalue "Texture" _texture)
  (`PrimitiveComponent.SetMaterial` _ingredientmesh 0 _returnvalue))

(fn `moveDown`
  (`self.K2_SetActorLocation` (`KismetMathLibrary.MakeVector` (.x (`self.K2_GetActorLocation`)) (.y (`self.K2_GetActorLocation`)) (- (.z (`self.K2_GetActorLocation`)) (`self.fallSpeed`)))))

(fn `randomRotation`
  (`self.K2_AddActorWorldRotation` (`KismetMathLibrary.MakeRotator` (`self.xRot`) (`self.yRot`) (`self.zRot`))))

(fn `UserConstructionScript`)