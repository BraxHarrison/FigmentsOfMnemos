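; Master actor for a garden map, which makes itself the player's view target and reacts to touches on its prop.
; BeginPlay caches the GameController and GameManager game instance, and a touch on Prop1 passes Prop1Name to ActivateProp.
; CleanupItem destroys the instantiated item if it is valid.
; ActivateProp, garden and prop initialization, and camera rotation are empty stubs here.
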(event `self.ReceiveBeginPlay`
  (bind _asgame_controller (cast `/Game/System/Control/GameController` (`GameplayStatics.GetPlayerController` 0)))
  (bind _output_get (set `self.gameController` _asgame_controller))
  (`PlayerController.SetViewTargetWithBlend` _output_get self 0.0 "VTBlend_Linear" 0.0 false)
  (`self.setGameManager`))

(event `self.ReceiveTick`
  (params (DeltaSeconds :type "Float (single-precision)")))

(event `self.Prop1.OnInputTouchBegin`
  (params (FingerIndex :type "ETouchIndex Enum" :default "Touch1") (TouchedComponent :type "PrimitiveComponent Object Reference"))
  (`self.activateProp` (`self.prop1Name`)))

(fn `activateProp`
  (params (propName :type String)))

(fn `cleanupItem`
  (bind _instantiateditem (`self.instantiatedItem`))
  (if (`KismetSystemLibrary.IsValid` _instantiateditem)
    (`/Game/Actors/Items/draggableItem_BP.destroyItem` _instantiateditem)))

(fn `initGarden`)

(fn `initProps`)

(fn `manageCameraRotation`)

(fn `setGameManager`
  (bind _asgame_manager (cast `/Game/System/Flow/GameManager` (`GameplayStatics.GetGameInstance`)))
  (set `self.GameManager` _asgame_manager))

(fn `UserConstructionScript`)