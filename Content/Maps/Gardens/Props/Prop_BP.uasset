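; Touchable garden prop (berries, per its message) that yields random inventory items once its drop interval has passed.
; InitProp stores the prop struct and GameManager, then applies the skeletal mesh and a dynamic material with the prop's texture.
; A touch compares time since last interaction to the interval, reporting unavailable or stamping the time and rolling the drop table once or twice.
; Drops play a shake animation and message, then the GameManager updates the garden's prop record.
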(event `self.ReceiveBeginPlay`)

(event `self.Mesh.OnInputTouchBegin`
  (params (FingerIndex :type "ETouchIndex Enum" :default "Touch1") (TouchedComponent :type "PrimitiveComponent Object Reference"))
  (`self.checkPropAvailable`)
  (`KismetSystemLibrary.PrintString` "At least try"))

(fn `activateProp`
  (bind _gamemanager (`self.GameManager`))
  (for _ (range (+ (`KismetMathLibrary.RandomIntegerInRange` 1 2) 1))
    (bind _result (`/Game/System/Functions/UniversalFunctions.RunRNG` (`.DropTable_16_F720D3CE49CFDF043C9226867772D1FF` (break `/Game/System/Types/Structs/Prop_STRUCT` (`self.propInfo`)))))
    (bind _itemout (`/Game/System/Flow/GameManager.LookupItemFromTable` _gamemanager _result))
    (`/Game/System/Flow/GameManager.AddItemToInventory` _gamemanager _itemout 1)
    (`SkeletalMeshComponent.PlayAnimation` (`self.Mesh`) "/Game/Maps/Props/BerryBush/Anims/Shake.Shake" false)
    (`/Game/System/Functions/UniversalFunctions.ReportMessage` (`KismetStringLibrary.Concat_StrStr` "Collected " " " (`.Name_2_6239F61F4E3C209977966C8BB4803326` (break `/Game/System/Types/Structs/Item_STRUCT` _itemout))) "NewEnumerator1" (`.Sprite_17_C67C2FD84EAB0B1EDE98EBA9AF8FA360` (break `/Game/System/Types/Structs/Item_STRUCT` _itemout))))
  (`/Game/System/Flow/GameManager.UpdatePropInGarden` _gamemanager (`self.propInfo`)))

(fn `checkPropAvailable`
  (bind _propinfo (`self.propInfo`))
  (bind ((`PropName_37_CF72D1E64C54C9FF3C6E81BB43C3B2F4` _propname) (`DropTable_16_F720D3CE49CFDF043C9226867772D1FF` _droptable) (`LastInteraction_34_5A27D60F465FFCA1A01244ACEB8E9F62` _lastinteraction) (`DropInterval_33_4E11D34649503DBE58E852A64B0F0F7E` _dropinterval)) (break `/Game/System/Types/Structs/Prop_STRUCT` _propinfo))
  (bind _timeelapsed (`/Game/System/Functions/UniversalFunctions.CheckTimeElapsed` _lastinteraction))
  (if (>= _dropinterval _timeelapsed)
    (`/Game/System/Functions/UniversalFunctions.ReportMessage` "There arent any berries right now.")
    (else
      (setmembers `/Game/System/Types/Structs/Prop_STRUCT` :`StructRef` _propinfo :`LastInteraction` (`KismetMathLibrary.Now`))
      (`self.activateProp`))))

(fn `initProp`
  (params (Prop :type "/Game/System/Types/Structs/Prop_STRUCT Structure") (GameManager :type "/Game/System/Flow/GameManager Object Reference"))
  (set `self.propInfo` Prop)
  (set `self.GameManager` GameManager)
  (`self.setupPropMesh`))

(fn `setupPropMesh`
  (bind _mesh (`self.Mesh`))
  (bind ((`Mesh_32_ED5FA4834F2CC00409FAEFB7084AA391` _mesh_2) (`Texture_31_A8BD89394FCA0446BD45E1BD5E9DEBDC` _texture) (`Skin_30_18187747422BAD873AF1C3B2274F38C1` _skin)) (break `/Game/System/Types/Structs/Prop_STRUCT` (`self.propInfo`)))
  (`SkinnedMeshComponent.SetSkinnedAssetAndUpdate` _mesh _mesh_2 true)
  (bind _returnvalue (`KismetMaterialLibrary.CreateDynamicMaterialInstance` _skin))
  (`MaterialInstanceDynamic.SetTextureParameterValue` _returnvalue "Texture" _texture)
  (`PrimitiveComponent.SetMaterial` _mesh 0 _returnvalue))

(fn `UserConstructionScript`)