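; Basic garden map actor, a child garden Blueprint with one harvestable berry prop that drops items on a timed cooldown.
; InitGarden and InitProps apply meshes and textured dynamic materials from GardenInfo, using only the first prop slot.
; ActivateProp checks time since last interaction, then rolls one or two drop-table items into the inventory with a shake animation and message.
; It saves the new interaction time to GardenInfo and the GameManager.
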(fn `activateProp`
  (params (propName :type String))
  (bind _gamemanager (`self.GameManager`))
  (bind _value (`BlueprintMapLibrary.Map_Find` (`.PropSlots_31_9450524D4FCC5441A7E82F8406FD5C75` (break `/Game/System/Types/Structs/Garden_STRUCT` (`self.gardenInfo`))) propName))
  (bind ((`PropName_37_CF72D1E64C54C9FF3C6E81BB43C3B2F4` _propname) (`DropTable_16_F720D3CE49CFDF043C9226867772D1FF` _droptable) (`LastInteraction_34_5A27D60F465FFCA1A01244ACEB8E9F62` _lastinteraction) (`DropInterval_33_4E11D34649503DBE58E852A64B0F0F7E` _dropinterval)) (break `/Game/System/Types/Structs/Prop_STRUCT` _value))
  (bind _timeelapsed (`/Game/System/Functions/UniversalFunctions.CheckTimeElapsed` _lastinteraction))
  (if (>= _dropinterval _timeelapsed)
    (`/Game/System/Functions/UniversalFunctions.ReportMessage` "There arent any berries right now.")
    (else
      (bind _structout (setmembers `/Game/System/Types/Structs/Prop_STRUCT` :`StructRef` _value :`LastInteraction` (`KismetMathLibrary.Now`)))
      (`BlueprintMapLibrary.Map_Add` (`.PropSlots_31_9450524D4FCC5441A7E82F8406FD5C75` (break `/Game/System/Types/Structs/Garden_STRUCT` (`self.gardenInfo`))) _propname _structout)
      (for _ (range (+ (`KismetMathLibrary.RandomIntegerInRange` 1 2) 1))
        (bind _result (`/Game/System/Functions/UniversalFunctions.RunRNG` _droptable))
        (bind _itemout (`/Game/System/Flow/GameManager.LookupItemFromTable` _gamemanager _result))
        (`/Game/System/Flow/GameManager.AddItemToInventory` _gamemanager _itemout 1)
        (`SkeletalMeshComponent.PlayAnimation` (`self.Prop1`) "/Game/Maps/Props/BerryBush/Anims/Shake.Shake" false)
        (`/Game/System/Functions/UniversalFunctions.ReportMessage` (`KismetStringLibrary.Concat_StrStr` "Collected " " " (`.Name_2_6239F61F4E3C209977966C8BB4803326` (break `/Game/System/Types/Structs/Item_STRUCT` _itemout))) "NewEnumerator1" (`.Sprite_17_C67C2FD84EAB0B1EDE98EBA9AF8FA360` (break `/Game/System/Types/Structs/Item_STRUCT` _itemout))))
      (`/Game/System/Flow/GameManager.UpdatePropInGarden` _gamemanager _structout)
      (`parent.activateProp` ""))))

(fn `initGarden`
  (bind (_name _backgroundsprite _backgroundzoom _figmentslots _propslots _skin _texture) (break `/Game/System/Types/Structs/Garden_STRUCT` (`self.gardenInfo`)))
  (bind _returnvalue (`KismetMaterialLibrary.CreateDynamicMaterialInstance` _skin))
  (`MaterialInstanceDynamic.SetTextureParameterValue` _returnvalue "Texture" _texture)
  (`PrimitiveComponent.SetMaterial` (`self.GardenMesh`) 0 _returnvalue)
  (`self.initProps`)
  (`parent.initGarden`))

(fn `initProps`
  (bind (_name _backgroundsprite _backgroundzoom _figmentslots _propslots) (break `/Game/System/Types/Structs/Garden_STRUCT` (`self.gardenInfo`)))
  (bind _keys (`BlueprintMapLibrary.Map_Keys` _propslots))
  (bind _output (`|GetArrayItem` _keys))
  (set `self.prop1Name` _output)
  (bind (_propname _droptable _proptype _lastinteraction _dropinterval _sprite _mesh _texture _skin) (break `/Game/System/Types/Structs/Prop_STRUCT` (`BlueprintMapLibrary.Map_Find` _propslots _output)))
  (`SkinnedMeshComponent.SetSkinnedAssetAndUpdate` (`self.Prop1`) _mesh true)
  (bind _returnvalue (`KismetMaterialLibrary.CreateDynamicMaterialInstance` _skin))
  (`MaterialInstanceDynamic.SetTextureParameterValue` _returnvalue "Texture" _texture)
  (`PrimitiveComponent.SetMaterial` (`self.Prop1`) 0 _returnvalue)
  (`parent.initProps`))

(fn `UserConstructionScript`)