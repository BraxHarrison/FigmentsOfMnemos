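; Garden Blueprint that hosts a Figment, a creature whose look and animation state come from its FigmentInfo struct.
; On BeginPlay it applies the struct's skeletal mesh, anim class and a textured dynamic material to FigmentMesh, then caches the GameHandler game mode.
; Helpers toggle the reach animation state and destroy the held item instance.
; Item acceptance, taking, eating and stat gain functions are empty stubs.
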(event `self.ReceiveBeginPlay`
  (`self.initFigment`)
  (bind _asgame_handler (cast `/Game/System/Flow/GameHandler` (`GameplayStatics.GetGameMode`)))
  (set `self.GameHandler` _asgame_handler))

(fn `[DEV]Print gained stat`
  (params (stat :type String) (PtGain :type Integer)))

(fn `addStatPoints`
  (params (Stat :type String) (Points :type Integer))
  (locals (ptsGained :type Integer) (statGained :type String) (statPtsToNextKey :type String) (statPtsKey :type String) (statsMap :type "Map of String to Object Object Reference") (newPtAmt :type Integer)))

(fn `eatFood`
  (params (food :type "/Game/System/Types/Item_STRUCT Structure"))
  (locals (statGained :type String)))

(fn `initFigment`
  (bind _figmentmesh (`self.FigmentMesh`))
  (bind ((`Grades_44_0FD2490D485E2BAFA9F4FCA90852C89B` _grades) (`RawStats_53_76D4C90545D0F557CBC565AF3C9295A2` _rawstats) (`Mesh_3_9607DBC34BC2F5BB7ED7F1BC401DC814` _mesh) (`AnimBlueprint_28_33CACA1A429DD8ACEA0C43957705C9F4` _animblueprint) (`Skin_22_C27CA512400D9FE23B7B4E9F6ABAB8A4` _skin) (`Texture_33_D64F4E0A49C23E408301C48BE5444740` _texture)) (break `/Game/System/Types/Figment_STRUCT` (`self.figmentInfo`)))
  (`|ExecutionSequence`
    (:`then_0`
      (`SkinnedMeshComponent.SetSkinnedAssetAndUpdate` _figmentmesh _mesh true)
      (`SkeletalMeshComponent.SetAnimInstanceClass` _figmentmesh _animblueprint))
    (:`then_1`
      (bind _returnvalue (`KismetMaterialLibrary.CreateDynamicMaterialInstance` _skin))
      (`MaterialInstanceDynamic.SetTextureParameterValue` _returnvalue "Texture" _texture)
      (`PrimitiveComponent.SetMaterial` (`self.FigmentMesh`) 0 _returnvalue))))

(fn `putAwayItem`
  (bind _iteminstance (`self.itemInstance`))
  (if (`KismetSystemLibrary.IsValid` _iteminstance)
    (`self.K2_DestroyActor` _iteminstance)))

(fn `takeItem`
  (params (item :type "/Game/System/Types/Item_STRUCT Structure")))

(fn `toggleFigmentReach`
  (bind _figmentinfo (`self.figmentInfo`))
  (if (`|EnumEquality` (`.AnimState_36_2BB6F3334D56C2EE90142595588FDDB7` (break `/Game/System/Types/Figment_STRUCT` _figmentinfo)) "NewEnumerator1")
    (setmembers `/Game/System/Types/Figment_STRUCT` :`StructRef` _figmentinfo :`AnimState` "NewEnumerator0")
    (else
      (setmembers `/Game/System/Types/Figment_STRUCT` :`StructRef` _figmentinfo :`AnimState` "NewEnumerator1"))))

(fn `UserConstructionScript`)

(fn `willFigmentAcceptItem`
  (params (NewParam :type "/Game/System/Types/Item_STRUCT Structure")))