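; Garden Blueprint that represents a Figment creature, building its mesh, anim class and textured dynamic material from FigmentInfo on BeginPlay.
; It toggles a reach animation state and accepts food only while stomach capacity allows.
; Eaten food adds points to one stat in a string-keyed map, rolling over into a level-up at the threshold.
; TakeItem then passes the updated Figment and garden name to GameHandler, the game mode.
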(event `self.ReceiveBeginPlay`
  (`self.initFigment`)
  (bind _asgame_handler (cast `/Game/System/Flow/GameHandler` (`GameplayStatics.GetGameMode`)))
  (set `self.GameHandler` _asgame_handler))

(fn `[DEV]Print gained stat`
  (params (stat :type String) (PtGain :type Integer))
  (`KismetSystemLibrary.PrintString` (`KismetStringLibrary.Concat_StrStr` "Gained " (`KismetStringLibrary.Conv_IntToString` PtGain) stat " points!" " Level: " (`KismetStringLibrary.Conv_IntToString` (`BlueprintMapLibrary.Map_Find` (`.Stats_10_D44B223F435FA506CFE9549967B720C4` (break `/Game/System/Types/Figment_STRUCT` (`self.figmentInfo`))) (`KismetStringLibrary.Concat_StrStr` stat "Lvl"))))))

(fn `addStatPoints`
  (params (Stat :type String) (Points :type Integer))
  (locals (ptsGained :type Integer) (statGained :type String) (statPtsToNextKey :type String) (statPtsKey :type String) (statsMap :type "Map of String to Object Object Reference") (newPtAmt :type Integer))
  (bind _returnvalue (`KismetStringLibrary.Concat_StrStr` (`local.statGained`) "Pts"))
  (bind _returnvalue_2 (`KismetStringLibrary.Concat_StrStr` (`local.statGained`) "Lvl"))
  (bind _returnvalue_3 (`KismetStringLibrary.Concat_StrStr` (`local.statGained`) "PtsToNext"))
  (bind _value (`BlueprintMapLibrary.Map_Find` (`local.statsMap`) _returnvalue_3))
  (set `local.statsMap` (`.Stats_10_D44B223F435FA506CFE9549967B720C4` (break `/Game/System/Types/Figment_STRUCT` (`self.figmentInfo`))))
  (set `local.ptsGained` Points)
  (set `local.statGained` Stat)
  (set `local.statPtsToNextKey` _returnvalue_3)
  (set `local.statPtsKey` _returnvalue)
  (set `local.newPtAmt` (+ (`BlueprintMapLibrary.Map_Find` (`local.statsMap`) _returnvalue) (`local.ptsGained`)))
  (`BlueprintMapLibrary.Map_Add` (`local.statsMap`) (`local.statPtsKey`) (`local.newPtAmt`))
  (if (>= (`local.newPtAmt`) _value)
    (`BlueprintMapLibrary.Map_Add` (`local.statsMap`) (`local.statPtsKey`) (mod (`local.newPtAmt`) _value))
    (`BlueprintMapLibrary.Map_Add` (`local.statsMap`) _returnvalue_2 (+ (`BlueprintMapLibrary.Map_Find` (`local.statsMap`) _returnvalue_2) 1)))
  (setmembers `/Game/System/Types/Figment_STRUCT` :`StructRef` (`self.figmentInfo`) :`Stats` (`local.statsMap`)))

(fn `eatFood`
  (params (food :type "/Game/System/Types/Item_STRUCT Structure"))
  (locals (statGained :type String))
  (bind ((`FoodType_8_99391E394D8F7F8B58CFFF81C80F51D1` _foodtype) (`AffectType_20_115D1CD9441DC3CCCC8A3B8A936EC04B` _affecttype) (`AffectAmt_11_04270E5845317F0DDC91E5A77DAB98AB` _affectamt)) (break `/Game/System/Types/Item_STRUCT` food))
  (bind _returnvalue (`KismetMathLibrary.FTrunc` _affectamt))
  (`|ExecutionSequence`
    (:`then_0`
      (switch `/Game/System/Types/AffectTypes` _affecttype
        (:`NewEnumerator0`
          (set `local.statGained` "Stamina"))
        (:`NewEnumerator2`
          (set `local.statGained` "Attack"))
        (:`NewEnumerator3`
          (set `local.statGained` "EnergyAttack"))
        (:`NewEnumerator4`
          (set `local.statGained` "Agility"))))
    (:`then_1`
      (`self.addStatPoints` (`local.statGained`) _returnvalue)
      (`self.[DEV]Print gained stat` (`local.statGained`) _returnvalue))))

(fn `initFigment`
  (bind _figmentmesh (`self.FigmentMesh`))
  (bind ((`Grades_44_0FD2490D485E2BAFA9F4FCA90852C89B` _grades) (`Mesh_3_9607DBC34BC2F5BB7ED7F1BC401DC814` _mesh) (`AnimBlueprint_28_33CACA1A429DD8ACEA0C43957705C9F4` _animblueprint) (`Skin_22_C27CA512400D9FE23B7B4E9F6ABAB8A4` _skin) (`Texture_33_D64F4E0A49C23E408301C48BE5444740` _texture)) (break `/Game/System/Types/Figment_STRUCT` (`self.figmentInfo`)))
  (`|ExecutionSequence`
    (:`then_0`
      (`SkinnedMeshComponent.SetSkinnedAssetAndUpdate` _figmentmesh _mesh true)
      (`SkeletalMeshComponent.SetAnimInstanceClass` _figmentmesh _animblueprint))
    (:`then_1`
      (bind _returnvalue (`KismetMaterialLibrary.CreateDynamicMaterialInstance` _skin))
      (`MaterialInstanceDynamic.SetTextureParameterValue` _returnvalue "Texture" _texture)
      (`PrimitiveComponent.SetMaterial` (`self.FigmentMesh`) 0 _returnvalue))))

(fn `putAwayItem`
  (`self.K2_DestroyActor` (`self.itemInstance`)))

(fn `takeItem`
  (params (item :type "/Game/System/Types/Item_STRUCT Structure"))
  (`|ExecutionSequence`
    (:`then_0`
      (switch `/Game/System/Types/ItemTypes` (`.Type_5_79367EC34A82EDDA80D3F188256374E0` (break `/Game/System/Types/Item_STRUCT` item))
        (:`NewEnumerator0`
          (`self.eatFood` item))))
    (:`then_1`
      (`/Game/System/Flow/GameHandler.updateExistingFigment` (`self.GameHandler`) (`self.figmentInfo`) (`.Name_9_8A7606234AC7A47F73F61FB0D6ED123B` (break `/Game/System/Types/Garden_STRUCT` (`self.gardenInfo`)))))))

(fn `toggleFigmentReach`
  (bind _figmentinfo (`self.figmentInfo`))
  (if (`|EnumEquality` (`.AnimState_36_2BB6F3334D56C2EE90142595588FDDB7` (break `/Game/System/Types/Figment_STRUCT` _figmentinfo)) "NewEnumerator1")
    (setmembers `/Game/System/Types/Figment_STRUCT` :`StructRef` _figmentinfo :`AnimState` "NewEnumerator0")
    (else
      (setmembers `/Game/System/Types/Figment_STRUCT` :`StructRef` _figmentinfo :`AnimState` "NewEnumerator1"))))

(fn `UserConstructionScript`)

(fn `willFigmentAcceptItem`
  (params (NewParam :type "/Game/System/Types/Item_STRUCT Structure"))
  (returns (willAccept :type Boolean))
  (bind ((`Type_5_79367EC34A82EDDA80D3F188256374E0` _type) (`Fillingness_34_3A01214A4EBB21EF88409D8D8EB8A1F9` _fillingness)) (break `/Game/System/Types/Item_STRUCT` NewParam))
  (bind ((`Stats_10_D44B223F435FA506CFE9549967B720C4` _stats)) (break `/Game/System/Types/Figment_STRUCT` (`self.figmentInfo`)))
  (switch `/Game/System/Types/ItemTypes` _type
    (:`NewEnumerator0`
      (if (> (`BlueprintMapLibrary.Map_Find` _stats "StomachCapacity") (+ (`BlueprintMapLibrary.Map_Find` _stats "StomachFullness") _fillingness))
        (return true)
        (else
          (return false))))))